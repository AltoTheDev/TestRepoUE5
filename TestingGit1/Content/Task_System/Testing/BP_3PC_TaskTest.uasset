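; BP_3PC_TaskTest is a test actor for the task system that gathers nearby tasks and lets the player pick one to perform.
; Begin and end overlap add and remove Task actors in a Tasks array.
; The cycle input advances a wrapping Select index, and the select input calls Do on that task and prints its name.
; An on-screen list highlighting the selection is disconnected, leaving the Tick loop empty.
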(event `self.ReceiveTick`
  (params (DeltaSeconds :type "Float (single-precision)"))
  (for (_array_element _array_index) (`self.Tasks`)
    _))

(event `self.ReceiveActorBeginOverlap`
  (params (OtherActor :type "Actor Object Reference"))
  (bind _astask (cast `/Game/Task_System/Task` OtherActor))
  (`KismetArrayLibrary.Array_Add` (`self.Tasks`) _astask))

(event `self.ReceiveActorEndOverlap`
  (params (OtherActor :type "Actor Object Reference"))
  (bind _astask (cast `/Game/Task_System/Task` OtherActor))
  (bind _returnvalue (`KismetArrayLibrary.Array_RemoveItem` (`self.Tasks`) _astask))
  (if (not _returnvalue)
    (`KismetSystemLibrary.PrintString` "What task?")))

(event `EnhancedInput|/Game/ThirdPerson/Input/Actions/IA_TaskCycle`
  (params (ActionValue :type Boolean) (ElapsedSeconds :type "Float (double-precision)") (TriggeredSeconds :type "Float (double-precision)") (InputAction :type "InputAction Object Reference" :default "/Game/ThirdPerson/Input/Actions/IA_TaskCycle.IA_TaskCycle"))
  (:`Triggered`
    (bind _result (`/Engine/EditorBlueprintResources/StandardMacros.IncrementInt` (`self.select`))
      (:`  `
        (bind _result_2 (`/Engine/EditorBlueprintResources/StandardMacros.DecrementInt` (`KismetArrayLibrary.Array_Length` (`self.Tasks`)))
          (:`  `
            (set `self.select` (`KismetMathLibrary.Wrap` _result 0 _result_2))))))))

(event `EnhancedInput|/Game/ThirdPerson/Input/Actions/IA_TaskSelect`
  (params (ActionValue :type Boolean) (ElapsedSeconds :type "Float (double-precision)") (TriggeredSeconds :type "Float (double-precision)") (InputAction :type "InputAction Object Reference" :default "/Game/ThirdPerson/Input/Actions/IA_TaskSelect.IA_TaskSelect"))
  (bind _output (`|GetArrayItem` (`self.Tasks`) (`self.select`)))
  (:`Triggered`
    (`/Game/Task_System/Task.Do` _output (`self.Details`))
    (`KismetSystemLibrary.PrintString` (`KismetTextLibrary.Conv_TextToString` (`.Name_4_F6B0B90143BE56AD5DB094B94C6FB187` (break `/Game/Task_System/TaskDetails` (`/Game/Task_System/Task.Details` _output)))))))

(fn `UserConstructionScript`
  (`parent.UserConstructionScript`))