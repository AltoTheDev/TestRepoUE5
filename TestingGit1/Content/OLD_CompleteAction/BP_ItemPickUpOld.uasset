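; Old item pickup actor meant to be destroyed after the player holds input for MaxHoldTime.
; Player overlap shows a WBP_BarOld progress widget and opens a gate, which closes on exit.
; The gate runs a retriggerable delay for destruction alongside a timer polled recursively to fill the bar.
; Nothing triggers the nodes that set IsHeld or enter the gate, so the hold never starts.
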(event `self.BoxCollision.OnComponentBeginOverlap`
  (params (OverlappedComponent :type "PrimitiveComponent Object Reference") (OtherActor :type "Actor Object Reference") (OtherComp :type "PrimitiveComponent Object Reference") (OtherBodyIndex :type Integer) (bFromSweep :type Boolean) (SweepResult :type "HitResult Structure (by ref)"))
  (cast `/Game/ThirdPerson/Blueprints/BP_Player` OtherActor)
  (`self.EnableInput` (`GameplayStatics.GetPlayerController` 0))
  (bind _returnvalue (`|CreateWidget` "/Game/OLD_CompleteAction/WBP_BarOld.WBP_BarOld_C"))
  (bind _output_get (set `self.Widget Ref` _returnvalue))
  (`UserWidget.AddToViewport` _output_get 0)
  (set `/Game/OLD_CompleteAction/WBP_BarOld.MaxTimeHeld` (`self.MaxHoldTime`) _output_get)
  (`/Engine/EditorBlueprintResources/StandardMacros.Gate` true :!via `Open` :!label _label
    (:`Exit`
      (`|ExecutionSequence`
        (:`then_0`
          (`KismetSystemLibrary.RetriggerableDelay` (`self.MaxHoldTime`))
          (if (`self.isHeld`)
            (`self.K2_DestroyActor`)))
        (:`then_1`
          (`self.Timer`)
          (`self.UpdateTimer`))))))

(event `StopTimer`
  (`KismetSystemLibrary.K2_PauseTimerHandle` (stale `Timer` _returnvalue)))

(event `Timer`
  (bind _returnvalue (`KismetSystemLibrary.K2_SetTimerDelegate` (delegate `Timer`) (`self.MaxHoldTime`))))

(event `self.BoxCollision.OnComponentEndOverlap`
  (params (OverlappedComponent :type "PrimitiveComponent Object Reference") (OtherActor :type "Actor Object Reference") (OtherComp :type "PrimitiveComponent Object Reference") (OtherBodyIndex :type Integer))
  (cast `/Game/ThirdPerson/Blueprints/BP_Player` OtherActor)
  (`self.EnableInput` (`GameplayStatics.GetPlayerController` 0))
  (`Widget.RemoveFromParent` (stale `self.BoxCollision.OnComponentBeginOverlap` _returnvalue))
  (goto _label :!via `Close`))

(event `UpdateTimer`
  (bind _widget_ref (`self.Widget Ref`))
  (if (`self.isHeld`)
    (set `/Game/OLD_CompleteAction/WBP_BarOld.TimeHeld` (`KismetSystemLibrary.K2_GetTimerElapsedTimeHandle` (stale `Timer` _returnvalue)) _widget_ref)
    (`KismetSystemLibrary.Delay` 0.1)
    (`self.UpdateTimer`)
    (else
      (`self.StopTimer`)
      (set `/Game/OLD_CompleteAction/WBP_BarOld.TimeHeld` 0.0 _widget_ref))))

(fn `UserConstructionScript`)